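; Hero head Blueprint for the dueling game that handles decapitation and its feedback.
; SetHeadMesh stores the mesh reference that Decapitate acts on, and an IsDecapitated getter exposes the resulting state.
; Decapitate sets that flag, enables physics on the head with a spin impulse, spawns blood and plays a random flesh-stab sound.
; It also shakes player 0's camera and rumbles both players' gamepads.
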(event EventDecapitate
  (Variables|Default|SetbIsDecapitated true)
  (Utilities|FlowControl|Sequence
    (:then_0
      ;[1 1 1] physics
      (Physics|SetSimulatePhysics (Variables|Default|GetHead%20Mesh) true)
      (Class|PrimitiveComponent|AddAngularImpulseinDegrees (Variables|Default|GetHead%20Mesh) (* (Math|Vector|GetRightVector (Variables|Default|GetHead%20Mesh)) 1e+03) "None" true))
    (:then_1
      ;[1 1 1] FX
      (Effects|SpawnEmitteratLocation "/Game/DuelingGame/FX/Hits/Blood/P_BloodBig.P_BloodBig" (+ (Transformation|GetWorldLocation (Variables|Default|GetDefaultSceneRoot)) "0,0.000000,10.000000")))
    (:then_2
      ;[1 1 1] audio
      (Audio|PlaySound2D (Utilities|Select :Index (Math|Random|RandomIntegerinRange 0 4) :Option%200 "/Game/Mediveal_Fight_Sounds_Pro/Cues/Sword_Stab_(Flesh)_-_5/Sword_Stab__Flesh__1_Cue.Sword_Stab__Flesh__1_Cue" :Option%201 "/Game/Mediveal_Fight_Sounds_Pro/Wavs/Sword_Stab_(Flesh)_-_5/Sword_Stab__Flesh__2.Sword_Stab__Flesh__2" :Option%202 "/Game/Mediveal_Fight_Sounds_Pro/Cues/Sword_Stab_(Flesh)_-_5/Sword_Stab__Flesh__3_Cue.Sword_Stab__Flesh__3_Cue" :Option%203 "/Game/Mediveal_Fight_Sounds_Pro/Cues/Sword_Stab_(Flesh)_-_5/Sword_Stab__Flesh__4_Cue.Sword_Stab__Flesh__4_Cue" :Option%204 "/Game/Mediveal_Fight_Sounds_Pro/Cues/Sword_Stab_(Flesh)_-_5/Sword_Stab__Flesh__5_Cue.Sword_Stab__Flesh__5_Cue") 1.0 1.0 0.0 0 0))
    (:then_3
      ;[1 1 1] cam shake
      (CameraShakes|StartCameraShake (Game|GetPlayerCameraManager 0) "/Game/DuelingGame/Core/Camera/Shake/CameraShake_Decapitate.CameraShake_Decapitate_C" 1.0 "CameraLocal" "0, 0, 0"))
    (:then_4
      ;[1 1 1] gamepad rumble
      (Game|Feedback|ClientPlayForceFeedback (Game|GetPlayerController 0) "/Game/DuelingGame/Core/GamePad/Rumble/Rumble_Hit.Rumble_Hit" "None" false false false)
      (Game|Feedback|ClientPlayForceFeedback (Game|GetPlayerController 1) "/Game/DuelingGame/Core/GamePad/Rumble/Rumble_Hit.Rumble_Hit" "None" false false false))))

(event EventSetHeadMesh
  (params (HeadMesh :type Static%20Mesh%20Component%20Object%20Reference%20%28by%20ref%29))
  (Variables|Default|SetHead%20Mesh HeadMesh))

(fn ConstructionScript)

(fn IsDecapitated
  (return (Variables|Default|GetbIsDecapitated)))