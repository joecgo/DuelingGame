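; BP_HeroArm drives a hero's weapon arm in the dueling game as a custom one-axis rotational physics simulation.
; Stick input becomes an eased force toward the target angle, mirrored by player side.
; Each tick applies damping, turns force over weapon mass into clamped velocity, then rotates the arm object.
; Weapon hits replace next-tick velocity using the opponent's momentum and block input during a stun scaled by impact speed.
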(event EventInitializeArm
  (params (MyHero :type BP%20Hero%20Object%20Reference%20%28by%20ref%29) (ObjToRotate :type Child%20Actor%20Component%20Object%20Reference%20%28by%20ref%29) (WeaponMass :type Float%20%28single-precision%29))
  (Variables|Default|SetMyHero MyHero)
  (Variables|Default|SetObjectToRotate ObjToRotate)
  (Variables|Default|SetWeaponMass WeaponMass))

(event EventTick
  (params (DeltaSeconds :type Float%20%28single-precision%29))
  (|ArmMotionUpdate DeltaSeconds))

(event EventWeaponHit
  (params (OtherMomentum :type Float%20%28single-precision%29))
  (CallFunction|ApplyWeaponHit OtherMomentum)
  (Variables|Default|SetbStunned true)
  (Utilities|FlowControl|Delay (Variables|Default|GetStunDuration))
  (Variables|Default|SetbStunned false))

(event EventArmInput
  (params (Input :type Vector%202D%20Structure))
  (CallFunction|CalculateArmInputForce Input))

(fn ConstructionScript)

(fn CalculateArmInputForce
  (params (ArmInput :type Vector%202D%20Structure))
  (bind _adjustedvalue (CallFunction|AdjustValueforPlayerSide (.x ArmInput)))
  (LocalVariables|SetLocalTargetDirection (Math|Vector|MakeVector _adjustedvalue (.y ArmInput) 0.0))
  (if (not (or (Math|Vector|VectorIsZero (LocalVariables|GetLocalTargetDirection)) (Variables|Default|GetbStunned)))
    (LocalVariables|SetLocalTargetAngle (Math|Trig|RadiansToDegrees (Class|KismetMathLibrary|VectorHeadingAngle (LocalVariables|GetLocalTargetDirection))))
    (Variables|Default|SetArmInputForce (Math|Interpolation|Ease "EaseIn" (Math|Float|Absolute(Float) (Utilities|AngleDifference (LocalVariables|GetLocalTargetAngle) (Variables|Default|GetAngle))) 0.0 (* (Math|Float|Sign(Float) (Utilities|AngleDifference (LocalVariables|GetLocalTargetAngle) (Variables|Default|GetAngle))) (Variables|Default|GetMaxArmInputForce)) 2.0))))

(fn StopArm
  (Variables|Default|SetVelocity 0.0)
  (Variables|Default|SetAcceleration 0.0)
  (Utilities|Array|Clear (Variables|Default|GetForces)))

(fn AddForce
  (params (Force :type Float%20%28single-precision%29) (DebugPrint :type Boolean) (Duration :type Float%20%28single-precision%29))
  (Utilities|Array|Add (Variables|Default|GetForces) (* Force Duration))
  (if DebugPrint
    (Development|PrintString (Utilities|String|Append "Added Force: " (Utilities|String|ToString(Float) Force)) true true "(R=0.000000,G=0.660000,B=1.000000,A=1.000000)" 0.0)))

(fn WrapRotationAngle
  (params (Angle :type Float%20%28single-precision%29))
  (bind _returnvalue (Math|Float|%(Float) Angle 3.6e+02))
  (bind _returnvalue_2 (+ _returnvalue 3.6e+02))
  (bind _returnvalue_3 (Math|Float|%(Float) _returnvalue_2 3.6e+02))
  (return (Math|Float|SelectFloat (- _returnvalue_3 3.6e+02) _returnvalue_3 (> _returnvalue_3 1.8e+02))))

(fn ApplyForces
  ;[1 1 1] convert forces into a change in acceleration
  (for _array_element (Variables|Default|GetForces)
    (Variables|Default|SetAcceleration (+ (Variables|Default|GetAcceleration) (/ _array_element (Variables|Default|GetWeaponMass)))))
  ;[1 1 1] clear forces from this tick
  (Utilities|Array|Clear (Variables|Default|GetForces)))

(fn TakeVelocityandPositionTimeStep
  (if (Variables|Default|GetbHitRegistered)
    ;[1 1 1] new velocity based on hit registered in previous tick
    (Variables|Default|SetVelocity (Variables|Default|GetVelocityAfterHit))
    (Variables|Default|SetbHitRegistered false)
    (else
      ;[1 1 1] Calculate velocity and new arm angle from acceleration
      (bind _output_get (Variables|Default|SetVelocity (Math|Float|Clamp(Float) (+ (* (Variables|Default|GetAcceleration) (Utilities|Time|GetWorldDeltaSeconds)) (Variables|Default|GetVelocity)) (* (Variables|Default|GetMaxVelocity) -1.0) (Variables|Default|GetMaxVelocity))))))
  (Variables|Default|SetAngle (+ (* _output_get (Utilities|Time|GetWorldDeltaSeconds)) (Variables|Default|GetAngle)))
  (Variables|Default|SetAcceleration 0.0)
  ;[1 1 1] Set rotation on arm object
  (Transformation|SetRelativeRotation (Variables|Default|GetObjectToRotate) (Math|Vector|RotatorfromAxisandAngle "0,1.000000, 0" (Variables|Default|GetAngle)) false false))

(fn ApplyDampening
  (Variables|Default|SetVelocity (* (Variables|Default|GetDamping) (Variables|Default|GetVelocity))))

(fn ApplyWeaponHit
  (params (OtherMomentum :type Float%20%28single-precision%29))
  (bind _output_get (Variables|Default|SetVelocityAfterHit (Utilities|ClamptoMaxVelocity (/ (* OtherMomentum (Variables|Default|GetHitEnergyConserved)) (Variables|Default|GetWeaponMass)))))
  (Variables|Default|SetbHitRegistered true)
  (Variables|Default|SetStunDuration (Math|Interpolation|Ease "EaseOut" (Math|Float|MapRangeClamped (Math|Float|Absolute(Float) _output_get) 0.0 (Variables|Default|GetMaxVelocity) 0.0 (Variables|Default|GetMaxStunDuration)) 0.0 (Variables|Default|GetMaxStunDuration) 1.5)))

(fn AdjustValueforPlayerSide
  (params (Value :type Float%20%28single-precision%29))
  ;[1 1 1] right player has values inverted so that mechanics can be mirrored
  (bind _leftmostplayer (Class|BPIGameMode|GetLeftMostPlayer(Message) (Game|GetGameMode)))
  (return (* (Math|Float|SelectFloat 1.0 -1.0 (== _leftmostplayer (Variables|Default|GetMyHero))) Value)))

(fn GetLeftMostPlayer
  (bind _outactors (Actor|GetAllActorsOfClass "/Game/DuelingGame/Core/Hero/BP_Hero.BP_Hero_C"))
  (LocalVariables|SetLocalHeroes _outactors)
  (if (== (Utilities|Array|Length (LocalVariables|GetLocalHeroes)) 0)
    (return 0 true)
    (else
      (return (Utilities|Array|Get(acopy) (LocalVariables|GetLocalHeroes) (Math|Integer|SelectInt 0 1 (< (.y (Transformation|GetWorldLocation (Variables|/Script/Engine.Actor|GetRootComponent (Utilities|Array|Get(acopy) (LocalVariables|GetLocalHeroes))))) (.y (Transformation|GetWorldLocation (Variables|/Script/Engine.Actor|GetRootComponent (Utilities|Array|Get(acopy) (LocalVariables|GetLocalHeroes) 1))))))) false))))

(fn GetArmAngle
  (return (Variables|Default|GetAngle)))

(fn GetMomentum
  (return (* (Variables|Default|GetVelocity) (Variables|Default|GetWeaponMass))))