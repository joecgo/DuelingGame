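; BP_Hero is the playable sword-fighting character in a side-on duel, with movement, jumping, directional arm control and impulse knockback on hits.
; RightArm, Sword and Head are child actors wired through messages, with sword mass passed to the arm on possession.
; Each tick disables control if the head reports decapitation, then eases rotation to lean with velocity and face by left/right position from the game mode.
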(event EventMoveInput
  (params (Forward :type Float%20%28single-precision%29))
  ;[1 1 1] Receiving input events from controller
  (if (Variables|Control|GetbControllable)
    (Class|PawnMovementComponent|AddInputVector (Variables|Character|GetCharacterMovement) (* (Class|KismetMathLibrary|VectorRight) Forward) false)))

(event EventTick
  (params (DeltaSeconds :type Float%20%28single-precision%29))
  ;[1 1 1] tick updates
  (CallFunction|UpdateControllableState)
  (CallFunction|UpdateCharacterRotation))

(event EventJumpInput
  ;[1 1 1] Receiving input events from controller
  (if (Variables|Control|GetbControllable)
    (Character|Jump)
    (Utilities|JumpSound)))

(event EventRightArmInput
  (params (Direction :type Vector%202D%20Structure))
  ;[1 1 1] Receiving input events from controller
  (if (Variables|Control|GetbControllable)
    (Class|BPIHeroArm|ArmInput(Message) (Variables|/Script/Engine.ChildActorComponent|GetChildActor (Variables|Default|GetRightArm)) Direction)))

(event EventTakeHit
  (params (Force :type Float%20%28single-precision%29) (Direction :type Vector :default "0, 0, 0"))
  ;[1 1 1] Take hit
  (Physics|AddImpulse (Variables|Character|GetCharacterMovement) (* Direction Force) true))

(event EventPossessed
  (params (NewController :type Controller%20Object%20Reference))
  ;[1 1 1] initial refs and variables for arm and head
  (bind _mass (Class|BPIHeroWeapon|GetMass(Message) (Variables|/Script/Engine.ChildActorComponent|GetChildActor (Variables|Default|GetSword))))
  (Class|BPIHeroArm|InitializeArm(Message) (Variables|/Script/Engine.ChildActorComponent|GetChildActor (Variables|Default|GetRightArm)) self (Variables|Default|GetRightArm) _mass)
  (Class|BPIHeroHead|SetHeadMesh(Message) (Variables|/Script/Engine.ChildActorComponent|GetChildActor (Variables|Default|GetHead)) (Variables|Default|GetStaticMesh_Head)))

(fn ConstructionScript
  (Class|BPIHeroWeapon|SetHero(Message) (Variables|/Script/Engine.ChildActorComponent|GetChildActor (Variables|Default|GetSword)) self)
  (bind _asbp_hero_arm (Utilities|Casting|CastToBP_HeroArm (Variables|/Script/Engine.ChildActorComponent|GetChildActor (Variables|Default|GetRightArm))))
  (Class|BPIHeroWeapon|SetArm(Message) (Variables|/Script/Engine.ChildActorComponent|GetChildActor (Variables|Default|GetSword)) _asbp_hero_arm))

(fn UpdateCharacterRotation
  ;[1 1 1] figure out if this character is on left or right
  (bind (_leftmostplayer _noplayers) (Class|BPIGameMode|GetLeftMostPlayer(Message) (Game|GetGameMode)))
  (if (not _noplayers)
    (LocalVariables|SetbIsLeftMostHero (== _leftmostplayer self))
    (Transformation|SetRelativeRotation (Variables|Transformation|GetRootComponent) (Math|Interpolation|Ease "EaseIn" 0.3 (Variables|/Script/Engine.SceneComponent|GetRelativeRotation (Variables|Transformation|GetRootComponent)) (Math|Rotator|MakeRotator 0.0 (.pitch (Math|Vector|RotatorfromAxisandAngle (Math|Vector|MakeVector 0.0 (Math|Float|SelectFloat 1.0 -1.0 (LocalVariables|GetbIsLeftMostHero)) 0.0) (* (.y (Pawn|Components|CharacterMovement|GetLastUpdateVelocity (Variables|Character|GetCharacterMovement))) 0.04))) (Math|Float|SelectFloat 9e+01 -9e+01 (LocalVariables|GetbIsLeftMostHero))) true) false false)))

(fn UpdateControllableState
  ;[1 1 1] disable control when decapitated
  (bind _bisdecapitated (Utilities|IsDecapitated))
  (Variables|Control|SetbControllable (not _bisdecapitated)))