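; BP_DuelCamera is the duel camera, which can switch to following a win-cam target.
; UseWinCam stores the target and enables following, which Tick then runs every frame through InterpToTarget.
; InterpToTarget eases the scene component toward the target's location plus an offset in X and Y at a fixed height, leaving rotation untouched.
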(event Custom|UseWinCam
  (params (WinCamTarget :type Actor%20Object%20Reference))
  (Variables|Default|SetWinCamTarget WinCamTarget)
  (Variables|Default|SetbUseTargetCam true))

(event EventTick
  (params (DeltaSeconds :type Float%20%28single-precision%29))
  (if (Variables|Default|GetbUseTargetCam)
    (CallFunction|InterptoTarget DeltaSeconds)))

(fn ConstructionScript)

(fn InterptoTarget
  (params (DeltaTime :type Float%20%28single-precision%29))
  (bind _wincamtarget (Variables|Default|GetWinCamTarget))
  (bind _wincamtargetoffset (Variables|Default|GetWinCamTargetOffset))
  (bind _rootcomponent (Variables|/Script/Engine.Actor|GetRootComponent _wincamtarget))
  (bind _returnvalue (Transformation|GetWorldLocation _rootcomponent))
  (bind _returnvalue_2 (+ _returnvalue _wincamtargetoffset))
  (Transformation|SetWorldLocation (Variables|Default|GetSceneComponent) (Math|Interpolation|VInterpTo (Transformation|GetWorldLocation (Variables|Default|GetSceneComponent)) (Math|Vector|MakeVector (.x _returnvalue_2) (.y _returnvalue_2) 1.2e+02) DeltaTime 3.0) false false))