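; Game mode for a two-player local duel, running the round loop from player setup through death to restart.
; On BeginPlay it registers the existing hero, creates a second local player and moves both to tagged PlayerStarts.
; Death events announce a winner through the GameState, with a RoundComplete flag blocking repeats.
; After a delay chosen by decapitation or knock-off, both heroes are destroyed, respawned as BP_Kevin, repossessed and repositioned.
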(event EventHeroDied
  (params (Hero :type BP%20Hero%20Object%20Reference) (Decapitated :type Boolean))
  (if (not (Variables|Default|GetRoundComplete))
    (Utilities|CompleteRound (Utilities|GetHeroIndex Hero) Decapitated)))

(event EventOtherHeroDied
  (params (Hero :type BP%20Hero%20Object%20Reference) (Decapitated :type Boolean))
  (if (not (Variables|Default|GetRoundComplete))
    (Utilities|CompleteRound (Utilities|GetOtherHeroIndex Hero) Decapitated)))

(event EventBeginPlay
  (CallFunction|StartGame)
  (CallFunction|StartRound))

(fn ConstructionScript)

(fn SpawnPlayer
  (params (PlayerIndex :type Integer) (PlayerCharacter :type BP%20Hero%20Object%20Reference))
  (return false))

(fn SetHeroStartPosition
  (params (Hero :type Actor%20Object%20Reference%20%28by%20ref%29) (StartPositionName :type Name))
  (bind _outactors (Actor|GetAllActorsOfClasswithTag "/Script/Engine.PlayerStart" StartPositionName))
  (Transformation|SetWorldTransform (Variables|/Script/Engine.Actor|GetRootComponent Hero) (Transformation|GetActorTransform (Utilities|Array|Get(acopy) _outactors)) false true))

(fn StartGame
  (Utilities|FlowControl|Sequence
    (:then_0
      ;[1 1 1] save ref to player1
      (bind _returnvalue (Actor|GetActorOfClass "/Game/DuelingGame/Core/Gameplay/BP_Hero.BP_Hero_C"))
      (Utilities|Array|SetArrayElem (Variables|Default|GetHeroes) 0 _returnvalue))
    (:then_1
      ;[1 1 1] create player 2
      (CallFunction|CreateNewPlayer 1))))

(fn CreateNewPlayer
  (params (PlayerIndex :type Integer))
  ;[1 1 1] create player
  (bind _returnvalue (Class|GameplayStatics|CreatePlayer PlayerIndex))
  (bind _asbp_hero (Utilities|Casting|CastToBP_Hero (Pawn|GetControlledPawn _returnvalue)))
  (Variables|/Game/DuelingGame/Core/Gameplay/BP_Hero.BP_Hero_C|SetPlayerIndex _asbp_hero PlayerIndex)
  ;[1 1 1] save player
  (Utilities|Array|SetArrayElem (Variables|Default|GetHeroes) PlayerIndex _asbp_hero))

(fn RestartRound
  (for (_array_element _array_index) (Variables|Default|GetHeroes)
    (Actor|DestroyActor _array_element)
    (CallFunction|RespawnHero _array_index))
  (CallFunction|StartRound))

(fn StartRound
  (bind _heroes (Variables|Default|GetHeroes))
  ;[1 1 1] start positions
  (CallFunction|SetHeroStartPosition (Utilities|Array|Get(acopy) _heroes) "Player1")
  (CallFunction|SetHeroStartPosition (Utilities|Array|Get(acopy) _heroes 1) "Player2"))

(fn RespawnHero
  (params (PlayerIndex :type Integer))
  (bind _returnvalue (Game|SpawnActorfromClass "/Game/DuelingGame/Characters/Kevin/BP_Kevin.BP_Kevin_C" (Math|Transform|MakeTransform "0, 0,150.000000" "0, 0, 0" "1,1,1") "Undefined" 0 0))
  (LocalVariables|SetLocalHero _returnvalue)
  (Variables|/Game/DuelingGame/Core/Gameplay/BP_Hero.BP_Hero_C|SetPlayerIndex (LocalVariables|GetLocalHero) PlayerIndex)
  (Utilities|Array|SetArrayElem (Variables|Default|GetHeroes) PlayerIndex (LocalVariables|GetLocalHero))
  (Pawn|Possess (Game|GetPlayerController PlayerIndex) (LocalVariables|GetLocalHero)))