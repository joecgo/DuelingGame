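; BP_Hero is the playable duelist, turning controller input events into movement along its right vector, jumps and right-arm aiming, with left-arm input left empty.
; Its right arm and sword are child actors: construction links the sword to hero and arm, and BeginPlay mirrors the arm by PlayerIndex.
; TakeHit applies knockback as a velocity impulse.
; An uncalled RotateInterpArm helper turns an arm toward TargetDirection at constant speed.
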(event EventMoveInput
  (params (Forward :type Float%20%28single-precision%29))
  ;[1 1 1] Receiving input events from controller
  (Class|PawnMovementComponent|AddInputVector (Variables|Character|GetCharacterMovement) (* (Class|KismetMathLibrary|VectorRight) Forward) false))

(event EventBeginPlay
  ;[1 1 1] flip x direction of arms based on player position
  (Class|BPIHeroArm|InitializeArm(Message) (Variables|/Script/Engine.ChildActorComponent|GetChildActor (Variables|Default|GetRightArm)) (== (Variables|Player|GetPlayerIndex) 1) (Variables|Default|GetRightArm)))

(event EventJumpInput
  ;[1 1 1] Receiving input events from controller
  (Character|Jump))

(event EventRightArmInput
  (params (Direction :type Vector%202D%20Structure))
  ;[1 1 1] Receiving input events from controller
  (Class|BPIHeroArm|ArmInput(Message) (Variables|/Script/Engine.ChildActorComponent|GetChildActor (Variables|Default|GetRightArm)) Direction))

(event EventLeftArmInput
  (params (Direction :type Vector%202D%20Structure))
  ;[1 1 1] Receiving input events from controller
)

(event EventTakeHit
  (params (Force :type Float%20%28single-precision%29) (Direction :type Vector :default "0, 0, 0"))
  (Physics|AddImpulse (Variables|Character|GetCharacterMovement) (* Direction Force) true))

(fn ConstructionScript
  (Class|BPIHeroWeapon|SetHero(Message) (Variables|/Script/Engine.ChildActorComponent|GetChildActor (Variables|Default|GetSword)) self)
  (bind _asbp_hero_arm (Utilities|Casting|CastToBP_HeroArm (Variables|/Script/Engine.ChildActorComponent|GetChildActor (Variables|Default|GetRightArm))))
  (Class|BPIHeroWeapon|SetArm(Message) (Variables|/Script/Engine.ChildActorComponent|GetChildActor (Variables|Default|GetSword)) _asbp_hero_arm))

(fn RotateInterpArm
  (params (Arm :type Scene%20Component%20Object%20Reference) (TargetDirection :type Vector%202D%20Structure) (InterpSpeed :type Float%20%28single-precision%29))
  (bind _playerindex (Variables|Player|GetPlayerIndex))
  (bind _returnvalue (== _playerindex 0))
  (bind _returnvalue_2 (Math|Float|SelectFloat 1.0 -1.0 _returnvalue))
  (bind _returnvalue_3 (* (.x TargetDirection) _returnvalue_2))
  (bind _returnvalue_4 (Math|Vector|MakeVector _returnvalue_3 (.y TargetDirection) 0.0))
  (if (Math|Vector|NotEqual(Vector) "0, 0, 0" _returnvalue_4 0.01)
    (Transformation|SetRelativeRotation Arm (Class|KismetMathLibrary|RInterptoConstant (Variables|/Script/Engine.SceneComponent|GetRelativeRotation Arm) (Math|Vector|RotatorfromAxisandAngle "0.000000,1.000000,0.000000" (Math|Trig|RadiansToDegrees (Class|KismetMathLibrary|VectorHeadingAngle _returnvalue_4))) (Utilities|Time|GetWorldDeltaSeconds) InterpSpeed) false false)))