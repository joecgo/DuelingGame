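; Hero arm for a dueling game that swings a given object around its Y axis using hand-rolled angular physics.
; Input direction, X-mirrored for player 2, becomes a target angle and an eased force signed by the angle difference.
; Each tick damps velocity, converts queued forces into acceleration by weapon weight, integrates clamped velocity and wraps the angle.
; Hits inject force, optionally hard-stopping the arm first.
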(event EventInitializeArm
  (params (MyHero :type BP%20Hero%20Object%20Reference%20%28by%20ref%29) (ObjToRotate :type Child%20Actor%20Component%20Object%20Reference%20%28by%20ref%29))
  (Variables|Default|SetMyHero MyHero)
  (Variables|Default|SetObjectToRotate ObjToRotate))

(event EventTick
  (params (DeltaSeconds :type Float%20%28single-precision%29))
  (|ArmMotionUpdate DeltaSeconds))

(event EventCreateHit
  (params (HardStop :type Boolean) (Force :type Float%20%28single-precision%29))
  (if HardStop
    (CallFunction|HardStopArm))
  (CallFunction|AddForce Force false 0.1))

(event EventArmInput
  (params (Input :type Vector%202D%20Structure))
  (CallFunction|CalculateArmInputForce Input))

(fn ConstructionScript)

(fn ManageHit
  (params (HardStop :type Boolean) (Force :type Float%20%28single-precision%29))
  (if HardStop
    _))

(fn CalculateArmInputForce
  (params (ArmInput :type Vector%202D%20Structure))
  (LocalVariables|SetLocalTargetDirection (Math|Vector|MakeVector (* (Math|Float|SelectFloat -1.0 1.0 (== (Variables|/Game/DuelingGame/Core/Gameplay/BP_Hero.BP_Hero_C|GetPlayerIndex (Variables|Default|GetMyHero)) 1)) (.x ArmInput)) (.y ArmInput) 0.0))
  (if (not (Math|Vector|VectorIsZero (LocalVariables|GetLocalTargetDirection)))
    (LocalVariables|SetLocalTargetAngle (Math|Trig|RadiansToDegrees (Class|KismetMathLibrary|VectorHeadingAngle (LocalVariables|GetLocalTargetDirection))))
    (Variables|Default|SetArmInputForce (Math|Interpolation|Ease "EaseIn" (Math|Float|Absolute(Float) (Utilities|AngleDifference (LocalVariables|GetLocalTargetAngle) (Variables|Default|GetAngle))) 0.0 (* (Math|Float|Sign(Float) (Utilities|AngleDifference (LocalVariables|GetLocalTargetAngle) (Variables|Default|GetAngle))) (Variables|Default|GetMaxArmInputForce)) 2.0))))

(fn HardStopArm
  (Variables|Default|SetVelocity 0.0)
  (Variables|Default|SetAcceleration 0.0)
  (Utilities|Array|Clear (Variables|Default|GetForces)))

(fn AddForce
  (params (Force :type Float%20%28single-precision%29) (DebugPrint :type Boolean) (Duration :type Float%20%28single-precision%29))
  (Utilities|Array|Add (Variables|Default|GetForces) (* Force Duration))
  (if DebugPrint
    (Development|PrintString (Utilities|String|Append "Added Force: " (Utilities|String|ToString(Float) Force)) true true "(R=0.000000,G=0.660000,B=1.000000,A=1.000000)" 0.0)))

(fn WrapRotationAngle
  (params (Angle :type Float%20%28single-precision%29))
  (bind _returnvalue (Math|Float|%(Float) Angle 3.6e+02))
  (bind _returnvalue_2 (+ _returnvalue 3.6e+02))
  (bind _returnvalue_3 (Math|Float|%(Float) _returnvalue_2 3.6e+02))
  (return (Math|Float|SelectFloat (- _returnvalue_3 3.6e+02) _returnvalue_3 (> _returnvalue_3 1.8e+02))))

(fn ApplyForces
  ;[1 1 1] convert forces into a change in acceleration
  (for _array_element (Variables|Default|GetForces)
    (Variables|Default|SetAcceleration (+ (Variables|Default|GetAcceleration) (/ _array_element (Variables|Default|GetWeaponWeight)))))
  ;[1 1 1] clear forces from this tick
  (Utilities|Array|Clear (Variables|Default|GetForces)))

(fn TakeVelocityandPositionTimeStep
  ;[1 1 1] Calculate velocity and new arm angle from acceleration
  (bind _output_get (Variables|Default|SetVelocity (Math|Float|Clamp(Float) (+ (* (Variables|Default|GetAcceleration) (Utilities|Time|GetWorldDeltaSeconds)) (Variables|Default|GetVelocity)) (* (Variables|Default|GetMaxVelocity) -1.0) (Variables|Default|GetMaxVelocity))))
  (Variables|Default|SetAngle (+ (* _output_get (Utilities|Time|GetWorldDeltaSeconds)) (Variables|Default|GetAngle)))
  (Variables|Default|SetAcceleration 0.0)
  ;[1 1 1] Set rotation on arm object
  (Transformation|SetRelativeRotation (Variables|Default|GetObjectToRotate) (Math|Vector|RotatorfromAxisandAngle "0,1.000000, 0" (Variables|Default|GetAngle)) false false))

(fn ApplyDampening
  (Variables|Default|SetVelocity (* (Variables|Default|GetDamping) (Variables|Default|GetVelocity))))

(fn GetArmAngle
  (return (Variables|Default|GetAngle)))