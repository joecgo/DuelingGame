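; Player controller for the dueling game that relays player input to the game state and to the controlled pawn.
; Menu select and back go to the game state as messages, with select carrying the controller ID and back a fixed zero.
; Movement, jump and two-axis arm input are forwarded to the pawn as messages.
; Cheat inputs use FlipFlops to toggle either hero between AI and player possession through BP_Duel_GameMode.
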(event Input|ActionEvents|InputActionJump
  (params (Key :type Key%20Structure :default "None"))
  ;[1 1 1] Passing input from player to the character they control
  (:Pressed
    (Class|BPIHero|JumpInput(Message) (Pawn|GetControlledPawn))))

(event Input|ActionEvents|InputActionCheat_ToggleP1AI
  (params (Key :type Key%20Structure :default "None"))
  ;[1 1 1] cheats
  (:Pressed
    (bind _asbp_game_mode (Utilities|Casting|CastToBP_Duel_GameMode (Game|GetGameMode)))
    (Utilities|FlowControl|FlipFlop
      (:A
        (Default|PossessHerobyAI _asbp_game_mode))
      (:B
        (Default|PossessHerobyPlayer _asbp_game_mode)))))

(event Input|ActionEvents|InputActionCheat_ToggleP2AI
  (params (Key :type Key%20Structure :default "None"))
  ;[1 1 1] cheats
  (:Pressed
    (bind _asbp_game_mode (Utilities|Casting|CastToBP_Duel_GameMode (Game|GetGameMode)))
    (Utilities|FlowControl|FlipFlop
      (:A
        (Default|PossessHerobyAI _asbp_game_mode 1))
      (:B
        (Default|PossessHerobyPlayer _asbp_game_mode 1)))))

(event Input|ActionEvents|InputActionMenu_Back
  (params (Key :type Key%20Structure :default "None"))
  (:Pressed
    (Class|BPICharacterSelectGameState|PlayerInputBack(Message) (Game|GetGameState))))

(event Input|ActionEvents|InputActionMenu_Select
  (params (Key :type Key%20Structure :default "None"))
  (:Pressed
    (Class|BPICharacterSelectGameState|PlayerInputSelect(Message) (Game|GetGameState) (Class|GameplayStatics|GetPlayerControllerID))))

(event Input|AxisEvents|InputAxisMove
  (params (AxisValue :type Float%20%28single-precision%29))
  ;[1 1 1] Passing input from player to the character they control
  (Class|BPIHero|MoveInput(Message) (Pawn|GetControlledPawn) AxisValue))

(event Input|AxisEvents|InputAxisLeftArmXAxis
  (params (AxisValue :type Float%20%28single-precision%29))
  ;[1 1 1] Passing input from player to the character they control
  (Class|BPIHero|LeftArmInput(Message) (Pawn|GetControlledPawn) (Math|Vector2D|MakeVector2D AxisValue (Input|AxisValues|GetLeftArmYAxis))))

(event Input|AxisEvents|InputAxisRightArmXAxis
  (params (AxisValue :type Float%20%28single-precision%29))
  ;[1 1 1] Passing input from player to the character they control
  (Class|BPIHero|RightArmInput(Message) (Pawn|GetControlledPawn) (Math|Vector2D|MakeVector2D AxisValue (Input|AxisValues|GetRightArmYAxis))))

(fn ConstructionScript)