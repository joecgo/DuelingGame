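; Player controller for the dueling game that relays player input to the character it controls.
; Move, RightArm and LeftArm axis values and Jump presses each go straight to the controlled pawn as input messages, leaving the response to the pawn.
; Forwarding has no validity check on the pawn, and the HasPawn graph holds only an unused IsValid check.
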(event Input|ActionEvents|InputActionJump
  (params (Key :type Key%20Structure))
  ;[1 1 1] Passing input from player to the character they control
  (:Pressed
    (Class|BPIHero|JumpInput(Message) (Pawn|GetControlledPawn))))

(event Input|AxisEvents|InputAxisMove
  (params (AxisValue :type Float%20%28single-precision%29))
  ;[1 1 1] Passing input from player to the character they control
  (Class|BPIHero|MoveInput(Message) (Pawn|GetControlledPawn) AxisValue))

(event Input|AxisEvents|InputAxisRightArm
  (params (AxisValue :type Float%20%28single-precision%29))
  ;[1 1 1] Passing input from player to the character they control
  (Class|BPIHero|RightArmInput(Message) (Pawn|GetControlledPawn) AxisValue))

(event Input|AxisEvents|InputAxisLeftArm
  (params (AxisValue :type Float%20%28single-precision%29))
  ;[1 1 1] Passing input from player to the character they control
  (Class|BPIHero|LeftArmInput(Message) (Pawn|GetControlledPawn) AxisValue))

(fn ConstructionScript)