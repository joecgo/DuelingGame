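; Game mode for a two-player local dueling game that sets up both heroes when play begins.
; InitializePlayers finds the existing BP_Hero as player one, then creates a second local player and assigns its pawn the second player index.
; Each hero teleports to a PlayerStart matched by tag and is written into the Heroes array.
; SpawnPlayer is an unused stub that returns false.
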(event EventBeginPlay
  (|InitializePlayers))

(fn ConstructionScript)

(fn SpawnPlayer
  (params (PlayerIndex :type Integer) (PlayerCharacter :type BP%20Hero%20Object%20Reference))
  (return false))

(fn SetHeroStartPosition
  (params (Hero :type Actor%20Object%20Reference%20%28by%20ref%29) (StartPositionName :type Name))
  (bind _outactors (Actor|GetAllActorsOfClasswithTag "/Script/Engine.PlayerStart" StartPositionName))
  (Transformation|SetWorldTransform (Variables|/Script/Engine.Actor|GetRootComponent Hero) (Transformation|GetActorTransform (Utilities|Array|Get(acopy) _outactors)) false true))