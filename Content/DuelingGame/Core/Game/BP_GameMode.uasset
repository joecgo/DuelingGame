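; Game mode for a local two-player duel that spawns both heroes, decides round winners and restarts rounds.
; At start it creates the second player, possesses each hero and teleports them to tagged PlayerStarts.
; Death events trigger a guarded completion sequence, with brief slow motion on decapitation.
; After a death-type-dependent delay, it destroys and respawns both heroes, then reports the winner to the GameState, which informs the HUD.
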(event EventHeroDied
  (params (Hero :type BP%20Hero%20Object%20Reference) (Decapitated :type Boolean))
  (if (not (Variables|Default|GetbRoundComplete))
    (Utilities|RoundCompletionSequence (Utilities|GetOtherHeroIndex Hero) Decapitated)))

(event EventOtherHeroDied
  (params (Hero :type BP%20Hero%20Object%20Reference) (Decapitated :type Boolean))
  (if (not (Variables|Default|GetbRoundComplete))
    (Utilities|RoundCompletionSequence (Utilities|GetHeroIndex Hero) Decapitated)))

(event EventBeginPlay
  (CallFunction|StartGame))

(fn ConstructionScript)

(fn SetHeroStartPositionfromPlayerStartTag
  (params (Hero :type Actor%20Object%20Reference%20%28by%20ref%29) (PlayerStartTag :type Name))
  (bind _outactors (Actor|GetAllActorsOfClasswithTag "/Script/Engine.PlayerStart" PlayerStartTag))
  (Transformation|SetWorldTransform (Variables|/Script/Engine.Actor|GetRootComponent Hero) (Transformation|GetActorTransform (Utilities|Array|Get(acopy) _outactors)) false true))

(fn StartGame
  (CallFunction|SpawnHero)
  (Class|GameplayStatics|CreatePlayer 1)
  (CallFunction|SpawnHero 1)
  (CallFunction|SetHeroStartPositions))

(fn SpawnHero
  (params (PlayerIndex :type Integer))
  (bind _returnvalue (Game|SpawnActorfromClass (Utilities|Select :Index PlayerIndex :Option%200 "/Game/DuelingGame/Characters/Kevin/BP_Kevin.BP_Kevin_C" :Option%201 "/Game/DuelingGame/Characters/Kevin/BP_KevinAlt.BP_KevinAlt_C") (Math|Transform|MakeTransform "0, 0,150.000000" "0, 0, 0" "1,1,1") "Undefined" 0 0))
  (bind _asbp_hero (Utilities|Casting|CastToBP_Hero _returnvalue))
  (Variables|/Game/DuelingGame/Core/Hero/BP_Hero.BP_Hero_C|SetPlayerIndex _asbp_hero PlayerIndex)
  (Utilities|Array|SetArrayElem (Variables|Default|GetHeroes) PlayerIndex _asbp_hero true)
  (Pawn|Possess (Game|GetPlayerController PlayerIndex) _asbp_hero))

(fn SetHeroStartPositions
  (bind _heroes (Variables|Default|GetHeroes))
  ;[1 1 1] start positions
  (CallFunction|SetHeroStartPositionfromPlayerStartTag (Utilities|Array|Get(acopy) _heroes) "Player1")
  (CallFunction|SetHeroStartPositionfromPlayerStartTag (Utilities|Array|Get(acopy) _heroes 1) "Player2"))

(fn KillHeroes
  (for _array_element (Variables|Default|GetHeroes)
    (Actor|DestroyActor _array_element)))

(fn GetLeftMostPlayer
  (bind _outactors (Actor|GetAllActorsOfClass "/Game/DuelingGame/Core/Hero/BP_Hero.BP_Hero_C"))
  (LocalVariables|SetLocalHeroes _outactors)
  (if (== (Utilities|Array|Length (LocalVariables|GetLocalHeroes)) 0)
    (return 0 true)
    (else
      (return (Utilities|Array|Get(acopy) (LocalVariables|GetLocalHeroes) (Math|Integer|SelectInt 0 1 (< (.y (Transformation|GetWorldLocation (Variables|/Script/Engine.Actor|GetRootComponent (Utilities|Array|Get(acopy) (LocalVariables|GetLocalHeroes))))) (.y (Transformation|GetWorldLocation (Variables|/Script/Engine.Actor|GetRootComponent (Utilities|Array|Get(acopy) (LocalVariables|GetLocalHeroes) 1))))))) false))))

(fn GetOtherHero
  (params (Hero :type BP%20Hero%20Object%20Reference%20%28by%20ref%29))
  (return (Utilities|Array|Get(acopy) (Variables|Default|GetHeroes) (Utilities|GetOtherHeroIndex Hero))))