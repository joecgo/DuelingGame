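; Game state Blueprint for the two-player character select screen, which starts the duel once both players are ready.
; It spawns the select HUD, tracks each player's menu state from select and back inputs, and updates the HUD on changes.
; When both are ready, it ignores those inputs, waits briefly, streams in the duel level, notifies the game mode, then unloads selection and destroys the HUD and itself.
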(event EventBeginPlay
  (bind _returnvalue (Game|SpawnActorfromClass "/Game/DuelingGame/HUD/CharacterSelect/BP_CharacterSelect_HUD.BP_CharacterSelect_HUD_C" (Math|Transform|MakeTransform "0, 0, 0" "0, 0, 0" "1,1,1") "Undefined" 0 0))
  (Variables|Default|SetHUD _returnvalue))

(event EventPlayerInputBack
  (params (PlayerIndex :type Integer))
  (if (not (Utilities|AllPlayersReady))
    (Utilities|SetMenuState PlayerIndex "NewEnumerator0")))

(event EventPlayerInputSelect
  (params (PlayerIndex :type Integer))
  (if (not (Utilities|AllPlayersReady))
    (Utilities|SetMenuState PlayerIndex "NewEnumerator1")))

(event EventPlayerIndexDirection
  (params (PlayerIndex :type Integer) (DirectionInput :type Vector%202D%20Structure)))

(fn ConstructionScript)