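; BP_GameState is the game state for a dueling game, tracking the scores of two players across rounds.
; On BeginPlay it spawns a BP_HUD actor and keeps a reference to it.
; RoundComplete takes the winner's index, increments that player's score through IncrementScore, then passes both scores to the HUD to update the display.
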(event EventBeginPlay
  (bind _returnvalue (Game|SpawnActorfromClass "/Game/DuelingGame/HUD/BP_HUD.BP_HUD_C" (Math|Transform|MakeTransform "0, 0, 0" "0, 0, 0" "1,1,1") "Undefined" 0 0))
  (Variables|Default|SetHUD _returnvalue))

(event EventRoundComplete
  (params (Winner :type Integer))
  (CallFunction|IncrementScore Winner)
  (Default|UpdateScore (Variables|Default|GetHUD) (Variables|Default|GetPlayer1Score) (Variables|Default|GetPlayer2Score)))

(fn ConstructionScript)

(fn IncrementScore
  (params (Winner :type Integer))
  (switch int Winner
    (:0
      (Math|Integer|IncrementInt (Variables|Default|GetPlayer1Score)))
    (:1
      (Math|Integer|IncrementInt (Variables|Default|GetPlayer2Score)))))