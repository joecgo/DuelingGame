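; Game mode for a two-player local sword duel, running character select, rounds and game over.
; It creates player two, then spawns both heroes at tagged PlayerStarts under player or AI control.
; Deaths trigger slow motion on decapitation, then either respawn both heroes and update the game state or show a winner cam and restart the level.
; It also plays cooldown-gated sword-clash effects, sound, camera shake and rumble.
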(event Custom|StartCharacterSelect
  (Game|LoadStreamLevel(byName) "CharacterSelect_Gameplay" true))

(event EventHeroDied
  (params (Hero :type BP%20Hero%20Object%20Reference) (Decapitated :type Boolean))
  (if (not (Variables|Default|GetbRoundComplete))
    (Utilities|RoundCompletionSequence (Utilities|GetOtherHeroIndex Hero) Decapitated)))

(event EventOtherHeroDied
  (params (Hero :type BP%20Hero%20Object%20Reference) (Decapitated :type Boolean))
  (if (not (Variables|Default|GetbRoundComplete))
    (Utilities|RoundCompletionSequence (Utilities|GetHeroIndex Hero) Decapitated)))

(event EventManageSwordonSwordFeedback
  (params (HitFeedbackInfo :type Hit%20Feedback%20Info%20Structure))
  (if (not (Variables|Default|GetbSwordOnSwordFeedbackActive))
    (Variables|Default|SetbSwordOnSwordFeedbackActive true)
    (CallFunction|CommitSwordonSwordFeedback HitFeedbackInfo)
    (Utilities|FlowControl|Delay (Variables|Default|GetSwordOnSwordFeedbackCooldownDuration))
    (Variables|Default|SetbSwordOnSwordFeedbackActive false)))

(event EventDuelStarted
  (Utilities|StartGame))

(event EventBeginPlay
  (Utilities|SetupPlayer2)
  (CallFunction|StartCharacterSelect))

(fn ConstructionScript)

(fn SetHeroStartPositionfromPlayerStartTag
  (params (Hero :type Actor%20Object%20Reference%20%28by%20ref%29) (PlayerStartTag :type Name))
  (bind _outactors (Actor|GetAllActorsOfClasswithTag "/Script/Engine.PlayerStart" PlayerStartTag))
  (Transformation|SetWorldTransform (Variables|/Script/Engine.Actor|GetRootComponent Hero) (Transformation|GetActorTransform (Utilities|Array|Get(acopy) _outactors)) false true))

(fn SpawnHero
  (params (PlayerIndex :type Integer))
  (bind _returnvalue (Game|SpawnActorfromClass (Utilities|Select :Index PlayerIndex :Option%200 "/Game/DuelingGame/Characters/Kevin/BP_Kevin.BP_Kevin_C" :Option%201 "/Game/DuelingGame/Characters/Kevin/BP_KevinAlt.BP_KevinAlt_C") (Math|Transform|MakeTransform "0, 0,150.000000" "0, 0, 0" "1,1,1") "Undefined" (Game|GetGameState) 0))
  (bind _asbp_hero (Utilities|Casting|CastToBP_Hero _returnvalue))
  (bind _output_get (LocalVariables|SetLocalHero _asbp_hero))
  (Utilities|Array|SetArrayElem (Variables|Default|GetAIControllers) PlayerIndex (Pawn|GetController _output_get))
  (Variables|/Game/DuelingGame/Core/Hero/BP_Hero.BP_Hero_C|SetPlayerIndex (LocalVariables|GetLocalHero) PlayerIndex)
  (Utilities|Array|SetArrayElem (Variables|Default|GetHeroes) PlayerIndex (LocalVariables|GetLocalHero) true)
  (if (Utilities|Array|Get(acopy) (Variables|Default|GetbUseAI) PlayerIndex)
    (Class|BPIAIController|StartBehavior(Message) (Utilities|Array|Get(acopy) (Variables|Default|GetAIControllers) PlayerIndex))
    (else
      (CallFunction|PossessHerobyPlayer PlayerIndex))))

(fn SetHeroStartPositions
  (bind _heroes (Variables|Default|GetHeroes))
  ;[1 1 1] start positions
  (CallFunction|SetHeroStartPositionfromPlayerStartTag (Utilities|Array|Get(acopy) _heroes) "Player1")
  (CallFunction|SetHeroStartPositionfromPlayerStartTag (Utilities|Array|Get(acopy) _heroes 1) "Player2"))

(fn KillHeroes
  (for _array_element (Variables|Default|GetHeroes)
    (Actor|DestroyActor _array_element)))

(fn PossessHerobyAI
  (params (PlayerIndex :type Integer))
  (Pawn|Possess (Utilities|Array|Get(acopy) (Variables|Default|GetAIControllers) PlayerIndex) (Utilities|Array|Get(acopy) (Variables|Default|GetHeroes) PlayerIndex))
  (Utilities|Array|SetArrayElem (Variables|Default|GetbUseAI) PlayerIndex true true)
  (Class|BPIAIController|StartBehavior(Message) (Utilities|Array|Get(acopy) (Variables|Default|GetAIControllers) PlayerIndex)))

(fn PossessHerobyPlayer
  (params (PlayerIndex :type Integer))
  (Pawn|Possess (Game|GetPlayerController PlayerIndex) (Utilities|Array|Get(acopy) (Variables|Default|GetHeroes) PlayerIndex))
  (Utilities|Array|SetArrayElem (Variables|Default|GetbUseAI) PlayerIndex false))

(fn CommitSwordonSwordFeedback
  (params (HitFeedbackInfo :type Hit%20Feedback%20Info%20Structure))
  (Utilities|FlowControl|Sequence
    (:then_0
      ;[1 1 1] FX
      (Effects|SpawnEmitteratLocation (.particlesystem HitFeedbackInfo) (.location HitFeedbackInfo)))
    (:then_1
      ;[1 1 1] sound
      (Audio|PlaySound2D (.sound HitFeedbackInfo) 1.0 (.pitchmultiplier HitFeedbackInfo) 0.0 0 0))
    (:then_2
      ;[1 1 1] cam shake
      (CameraShakes|StartCameraShake (Game|GetPlayerCameraManager 0) "/Game/DuelingGame/Core/Camera/Shake/CameraShake_SwordHit.CameraShake_SwordHit_C" (.intensityscale HitFeedbackInfo) "CameraLocal" "0, 0, 0"))
    (:then_3
      ;[1 1 1] gamepad rumble
      (Game|Feedback|ClientPlayForceFeedback (Game|GetPlayerController 0) (.rumbleeffect HitFeedbackInfo) "None" false true false)
      (Game|Feedback|ClientPlayForceFeedback (Game|GetPlayerController 1) (.rumbleeffect HitFeedbackInfo) "None" false true false))))

(fn GetLeftMostPlayer
  (bind _outactors (Actor|GetAllActorsOfClass "/Game/DuelingGame/Core/Hero/BP_Hero.BP_Hero_C"))
  (LocalVariables|SetLocalHeroes _outactors)
  (if (< (Utilities|Array|Length (LocalVariables|GetLocalHeroes)) 2)
    (return 0 true)
    (else
      (return (Utilities|Array|Get(acopy) (LocalVariables|GetLocalHeroes) (Math|Integer|SelectInt 0 1 (< (.y (Transformation|GetWorldLocation (Variables|/Script/Engine.Actor|GetRootComponent (Utilities|Array|Get(acopy) (LocalVariables|GetLocalHeroes))))) (.y (Transformation|GetWorldLocation (Variables|/Script/Engine.Actor|GetRootComponent (Utilities|Array|Get(acopy) (LocalVariables|GetLocalHeroes) 1))))))) false))))

(fn GetOtherHero
  (params (Hero :type BP%20Hero%20Object%20Reference%20%28by%20ref%29))
  (return (Utilities|Array|Get(acopy) (Variables|Default|GetHeroes) (Utilities|GetOtherHeroIndex Hero))))