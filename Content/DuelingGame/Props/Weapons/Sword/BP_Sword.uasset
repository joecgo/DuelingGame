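; BP_Sword is the sword weapon in the dueling game, hitting any hero it overlaps other than its own wielder.
; External setters supply the owning hero and the arm that swings it.
; On overlap it sends the other hero a hit message with force scaled from the arm's velocity and weapon weight.
; Horizontal knockback direction comes from the wielder's player index, with a fixed upward component.
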(event EventSetHero
  (params (Hero :type BP%20Hero%20Object%20Reference))
  (Variables|Default|SetMyHero Hero))

(event EventSetArm
  (params (Arm :type BP%20Hero%20Arm%20Object%20Reference))
  (Variables|Default|SetMyArm Arm))

(event Collision|EventActorBeginOverlap
  (params (OtherActor :type Actor%20Object%20Reference))
  (bind _asbp_hero (Utilities|Casting|CastToBP_Hero OtherActor))
  (if (!= _asbp_hero (Variables|Default|GetMyHero))
    (CallFunction|OtherHeroHit _asbp_hero)))

(fn ConstructionScript)

(fn OtherHeroHit
  (params (OtherHero :type BP%20Hero%20Object%20Reference))
  (bind _myarm (Variables|Default|GetMyArm))
  (Class|BPIHero|TakeHit(Message) OtherHero (Math|Float|Absolute(Float) (* (Variables|/Game/DuelingGame/Core/Gameplay/BP_HeroArm.BP_HeroArm_C|GetVelocity _myarm) (Variables|/Game/DuelingGame/Core/Gameplay/BP_HeroArm.BP_HeroArm_C|GetWeaponWeight _myarm) (Variables|Default|GetHitForceScalar))) (Math|Vector|MakeVector 0.0 (Math|Float|SelectFloat 1.0 -1.0 (== (Variables|/Game/DuelingGame/Core/Gameplay/BP_Hero.BP_Hero_C|GetPlayerIndex (Variables|Default|GetMyHero)) 0)) 1.0)))