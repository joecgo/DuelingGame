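; BP_HeroHead manages a hero's head in the dueling game and handles its decapitation.
; SetHeadMesh stores the mesh that represents the head.
; Decapitate sets the IsDecapitated flag, turns on physics simulation for that mesh and spins it with an angular impulse around its right vector.
; The IsDecapitated function exposes that state to callers.
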(event EventDecapitate
  (bind _head_mesh (Variables|Default|GetHead%20Mesh))
  (Variables|Default|SetbIsDecapitated true)
  (Physics|SetSimulatePhysics (Variables|Default|GetHead%20Mesh) true)
  (Class|PrimitiveComponent|AddAngularImpulseinDegrees _head_mesh (* (Math|Vector|GetRightVector _head_mesh) 1e+03) "None" true))

(event EventSetHeadMesh
  (params (HeadMesh :type Static%20Mesh%20Component%20Object%20Reference%20%28by%20ref%29))
  (Variables|Default|SetHead%20Mesh HeadMesh))

(fn ConstructionScript)

(fn IsDecapitated
  (return (Variables|Default|GetbIsDecapitated)))